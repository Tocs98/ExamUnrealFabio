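; Explosive actor that destroys itself when a countdown runs out, with no damage or effects in its graph.
; BeginPlay starts a self-calling custom event that lowers CountDownTime by a fixed step, waits on a matching Delay, and repeats until zero or below.
; An overlap on the static mesh calls the same event, so each overlap takes an extra step off the countdown.
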(event OnComponentBeginOverlap(StaticMeshComponent)
  (params (OverlappedComponent :type Primitive%20Component%20Object%20Reference) (OtherActor :type Actor%20Object%20Reference) (OtherComp :type Primitive%20Component%20Object%20Reference) (OtherBodyIndex :type Integer) (bFromSweep :type Boolean) (SweepResult :type Hit%20Result%20Structure%20%28by%20ref%29))
  (CallFunction|ExpEVT))

(event Custom|expEVT
  (Variables|Default|SetcountDownTime (- (Variables|Default|GetcountDownTime) 0.2))
  (Math|Float|CompareFloat (Variables|Default|GetcountDownTime) 0.0
    (:>
      (Utilities|FlowControl|Delay 0.2)
      (CallFunction|ExpEVT))
    (:==
      (Actor|DestroyActor :!label _label))
    (:<
      (goto _label))))

(event EventBeginPlay
  (CallFunction|ExpEVT))

(event Collision|EventActorBeginOverlap
  (params (OtherActor :type Actor%20Object%20Reference)))

(event EventTick
  (params (DeltaSeconds :type Float%20%28single-precision%29)))

(fn ConstructionScript)