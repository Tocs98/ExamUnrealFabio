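; Platform actor that makes one trip out and back along its local X axis, starting on BeginPlay.
; PlatfMove and ReversePlat call themselves through short Delays, stepping a CurrentDistance counter up past Distance, then down to zero, where movement stops.
; Each step uses the counter itself as the offset delta, so the platform speeds up outbound and slows down returning.
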(event Custom|platfMove
  (Variables|Default|SetcurrentDistance (+ (Variables|Default|GetcurrentDistance) 1.0))
  (Math|Float|CompareFloat (Variables|Default|GetcurrentDistance) (Variables|Default|Getdistance)
    (:>
      (CallFunction|ReversePlat))
    (:==
      (Transformation|AddActorLocalOffset (Math|Vector|MakeVector (Variables|Default|GetcurrentDistance) 0.0 0.0) false false :!label _label)
      (Utilities|FlowControl|Delay 0.01)
      (CallFunction|PlatfMove))
    (:<
      (goto _label))))

(event Custom|reversePlat
  (Variables|Default|SetcurrentDistance (- (Variables|Default|GetcurrentDistance) 1.0))
  (Math|Float|CompareFloat (Variables|Default|GetcurrentDistance) 0.0
    (:>
      (Transformation|AddActorLocalOffset (Math|Vector|MakeVector (* (Variables|Default|GetcurrentDistance) -1.0) 0.0 0.0) false false)
      (Utilities|FlowControl|Delay 0.01)
      (CallFunction|ReversePlat))))

(event EventBeginPlay
  (CallFunction|PlatfMove))

(event Collision|EventActorBeginOverlap
  (params (OtherActor :type Actor%20Object%20Reference)))

(fn ConstructionScript)